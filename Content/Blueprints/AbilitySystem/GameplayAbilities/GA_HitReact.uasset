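; GA_HitReact is a gameplay ability that plays a hit reaction montage on its avatar.
; On activation it applies GE_HitReact to the owner, stores the handle, and gets the montage from the avatar through CombatInterface.
; When the montage completes, is interrupted or is cancelled, it removes the effect by handle and ends the ability, with debug prints along the way.
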(event `self.K2_ActivateAbility`
  (bind _returnvalue (`self.BP_ApplyGameplayEffectToOwner` "/Game/Blueprints/AbilitySystem/GameplayEffects/GE_HitReact.GE_HitReact_C"))
  (set `self.ActiveGE_HitReact` _returnvalue)
  (bind _ascombat_interface (cast `CombatInterface` (`self.GetAvatarActorFromActorInfo`)))
  (bind _returnvalue_2 (`CombatInterface.GethitReactMontage` _ascombat_interface))
  (`KismetSystemLibrary.PrintString` (`KismetSystemLibrary.GetObjectName` _returnvalue_2))
  (`AbilityTask_PlayMontageAndWait.CreatePlayMontageAndWaitProxy` "None" _returnvalue_2 1.0 "None" false
    (:`OnCompleted`
      (`KismetSystemLibrary.PrintString` "MontageCompleted"))
    (:`OnInterrupted`
      (`KismetSystemLibrary.PrintString` "MontageINT"))
    (:`OnCancelled`
      (`KismetSystemLibrary.PrintString` "MontageCANCELLED")))
  (`self.BP_RemoveGameplayEffectFromOwnerWithHandle` (`self.ActiveGE_HitReact`))
  (`self.K2_EndAbility`))